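; Player SWAT character with Enhanced Input movement, sprint and rifle aiming, plus HUD widgets for health, ammo and crosshair.
; BeginPlay attaches BP_Weapon to a hand socket; Tick updates the left-hand socket position and ammo state.
; Aiming-only fire plays montage, effects and a camera-then-muzzle double line trace, whose final hit is unused.
; Health changes via an add event or key 1 calling ACHealth.
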(event `self.ReceiveBeginPlay`
  (`|ExecutionSequence`
    (:`then_1`
      ;[0.3423 1 0] Отображения главного виджета игры
      (bind _returnvalue (`|CreateWidget` "/Game/Data/Widgets/WBP_CrossHair.WBP_CrossHair_C"))
      (set `self.WBP_Crosshair` _returnvalue)
      (bind _returnvalue_2 (`|CreateWidget` "/Game/Data/Widgets/WBP_MainWidget.WBP_MainWidget_C"))
      (bind _output_get (set `self.ABP_Mainwidget` _returnvalue_2))
      (`UserWidget.AddToViewport` _output_get 0))
    (:`then_2`
      ;[0 1 0.9532] Спавн оружия в руке
      (bind _returnvalue_3 (`|SpawnActorFromClass` "/Game/FPS_Weapon_Bundle/BP_Weapon.BP_Weapon_C" (`SceneComponent.GetSocketTransform` (`self.Mesh`) "WeaponSocket" "RTS_World") "Undefined" "MultiplyWithRoot" null null))
      (bind _output_get_2 (set `self.BP_Weapon` _returnvalue_3))
      (`self.K2_AttachToComponent` _output_get_2 (`self.Mesh`) "WeaponSocket" "SnapToTarget" "SnapToTarget" "SnapToTarget" true))
    (:`then_3`
      ;[0.5016 0.4099 1] Перемещение персонажа и камеры
      (bind _asplayer_controller (cast `PlayerController` (`self.GetController`)))
      (`EnhancedInputSubsystemInterface.AddMappingContext` (pcsubsystem `EnhancedInputLocalPlayerSubsystem` _asplayer_controller) "/Game/Data/Inputs/IMC_Default.IMC_Default" 0 (struct)))))

(event `/Game/Data/BPI_TakeHealth.Func_AddHealth`
  (params (Health :type "Float (double-precision)"))
  ;[0.3385 0.2675 0.006659] Логика увеличения и уменьшения HP
  (bind _output_get (set `self.Health` (+ Health (`self.Health`))))
  (`ProgressBar.SetPercent` (`/Game/Data/Widgets/WBP_MainWidget.PG_HealthBar` (`self.ABP_Mainwidget`)) (`KismetMathLibrary.FClamp` _output_get)))

(event `Key|One`
  (params (Key :type "Key Structure"))
  ;[0.3385 0.2675 0.006659] Логика увеличения и уменьшения HP
  (:`Pressed`
    (bind _health (`/Game/Data/AC_Health.Func_Hit` (`self.AC_Health`)))
    (bind _output_get (set `self.Health` _health))
    (`ProgressBar.SetPercent` (`/Game/Data/Widgets/WBP_MainWidget.PG_HealthBar` (`self.ABP_Mainwidget`)) _output_get)))

(event `EnhancedInput|/Game/Data/Inputs/IA_Move`
  (params (ActionValue :type "Vector2D Structure") (ElapsedSeconds :type "Float (double-precision)") (TriggeredSeconds :type "Float (double-precision)") (InputAction :type "InputAction Object Reference" :default "/Game/Data/Inputs/IA_Move.IA_Move"))
  (bind (_returnvalue_roll _returnvalue_pitch _returnvalue_yaw) (`KismetMathLibrary.BreakRotator` (`self.GetControlRotation`)))
  (bind (_returnvalue_roll_2 _returnvalue_pitch_2 _returnvalue_yaw_2) (`KismetMathLibrary.BreakRotator` (`self.GetControlRotation`)))
  ;[0.5016 0.4099 1] Перемещение персонажа и камеры
  ;;[1 0.3761 0.236] Перемещение вперд назад влево вправо
  (:`Triggered`
    (`self.AddMovementInput` (`KismetMathLibrary.GetRightVector` (`KismetMathLibrary.MakeRotator` _returnvalue_roll 0.0 _returnvalue_yaw)) ActionValue_X)
    (`self.AddMovementInput` (`KismetMathLibrary.GetForwardVector` (`KismetMathLibrary.MakeRotator` 0.0 0.0 _returnvalue_yaw_2)) ActionValue_Y)))

(event `self.ReceiveTick`
  (params (DeltaSeconds :type "Float (single-precision)"))
  (bind _returnvalue_location (`KismetMathLibrary.BreakTransform` (`SceneComponent.GetSocketTransform` (`/Game/FPS_Weapon_Bundle/BP_Weapon.Weapon` (`self.BP_Weapon`)) "LeftHandSocketpos" "RTS_World")))
  ;[1 0.9413 0.5395] Покадровая проверка есть ли у нас потроны
  (set `self.LeftHandPos` _returnvalue_location)
  (if (== 0 (`self.Ammo`))
    (set `self.bCanShoot` false)
    (else
      (set `self.bCanShoot` true)))
  (`TextBlock.SetText` (`/Game/Data/Widgets/WBP_MainWidget.Ammo` (`self.ABP_Mainwidget`)) (`KismetTextLibrary.Conv_IntToText` (`self.Ammo`))))

(event `EnhancedInput|/Game/Data/Inputs/IA_Look`
  (params (ActionValue :type "Vector2D Structure") (ElapsedSeconds :type "Float (double-precision)") (TriggeredSeconds :type "Float (double-precision)") (InputAction :type "InputAction Object Reference" :default "/Game/Data/Inputs/IA_Look.IA_Look"))
  ;[0.5016 0.4099 1] Перемещение персонажа и камеры
  ;;[1 0.3604 0.9248] Камера
  (:`Triggered`
    ;;;[0.4022 0.5869 1] Влево Вправо
    (`self.AddControllerYawInput` ActionValue_X)
    ;;;[0.4022 0.5869 1] Вверх Вниз
    (`self.AddControllerPitchInput` ActionValue_Y)))

(event `EnhancedInput|/Game/Data/Inputs/IA_Shoot`
  (params (ActionValue :type Boolean) (ElapsedSeconds :type "Float (double-precision)") (TriggeredSeconds :type "Float (double-precision)") (InputAction :type "InputAction Object Reference" :default "/Game/Data/Inputs/IA_Shoot.IA_Shoot"))
  ;[0.09423 0.1002 1] Стрельба
  (:`Triggered`
    (`/Engine/EditorBlueprintResources/StandardMacros.DoOnce` false :!label _label
      (:`Completed`
        (if (`self.bIsAiming`)
          (if (`self.bCanShoot`)
            (`|PlayMontage` (`self.Mesh`) "/Game/MainCharacter/Anims/Firing_Rifle_Montage.Firing_Rifle_Montage"
              (:`then`
                (`/Game/FPS_Weapon_Bundle/BP_Weapon.SpawnLight` (`self.BP_Weapon`))
                (`GameplayStatics.SpawnSound2D` "/Game/Data/Sounds/AK_Sound_Wav.AK_Sound_Wav" 1.0 (`KismetMathLibrary.FClamp` (`KismetMathLibrary.RandomFloat`) 0.8 1.1) 0.0 null)
                (`AddComponent|NODE_AddCameraShakeSourceComponent-0` :`RelativeTransform` (`SceneComponent.GetRelativeTransform` (`self.Camera`)))
                (`self.AmmoCounter`)
                (`self.LineTrace`)
                (`KismetSystemLibrary.Delay` 0.1)
                (goto _label :!via `Reset`)))
            (else
              (`GameplayStatics.SpawnSound2D` "/Game/Data/Sounds/EmptyAK.EmptyAK" 1.0 (`KismetMathLibrary.FClamp` (`KismetMathLibrary.RandomFloat`) 0.7 1.2) 0.0 null)))))))
  (:`Completed`
    (`self.StopAnimMontage` "/Game/MainCharacter/Anims/Firing_Rifle_Montage.Firing_Rifle_Montage")
    (goto _label :!via `Reset`)))

(event `EnhancedInput|/Game/Data/Inputs/IA_Aiming`
  (params (ActionValue :type Boolean) (ElapsedSeconds :type "Float (double-precision)") (TriggeredSeconds :type "Float (double-precision)") (InputAction :type "InputAction Object Reference" :default "/Game/Data/Inputs/IA_Aiming.IA_Aiming"))
  (bind _charactermovement (`self.CharacterMovement`))
  (bind _wbp_crosshair (`self.WBP_Crosshair`))
  (bind _wbp_crosshair_2 (`self.WBP_Crosshair`))
  (bind _camera (`self.Camera`))
  (bind (_relativelocation_x _relativelocation_y _relativelocation_z) (`KismetMathLibrary.BreakVector` (`SceneComponent.RelativeLocation` _camera)))
  ;[1 0.06778 0.3511] Прицеливание
  (:`Started`
    (set `self.bIsAiming` true)
    (set `CharacterMovementComponent.bOrientRotationToMovement` false _charactermovement)
    (set `self.bUseControllerRotationYaw` true)
    (`UserWidget.AddToViewport` _wbp_crosshair 0)
    (bind (_direction _zoom) (`Timeline|TL_Aim_Template` :!label _label_2)
      (:`Update`
        (`SceneComponent.K2_SetRelativeLocation` _camera (`KismetMathLibrary.MakeVector` (`KismetMathLibrary.Lerp` 0.0 75.0 _zoom) _relativelocation_y _relativelocation_z) false false)
        (`UserWidget.PlayAnimationForward` _wbp_crosshair_2 (`/Game/Data/Widgets/WBP_CrossHair.ZoomCrossHair` _wbp_crosshair_2) 1.0 false))))
  (:`Canceled`
    (set `self.bIsAiming` false :!label _label_3)
    (set `CharacterMovementComponent.bOrientRotationToMovement` true _charactermovement)
    (set `self.bUseControllerRotationYaw` false)
    (`Widget.RemoveFromParent` _wbp_crosshair)
    (goto _label_2 :!via `Reverse`))
  (:`Completed`
    (goto _label_3)))

(event `EnhancedInput|/Game/Data/Inputs/IA_Sprint`
  (params (ActionValue :type Boolean) (ElapsedSeconds :type "Float (double-precision)") (TriggeredSeconds :type "Float (double-precision)") (InputAction :type "InputAction Object Reference" :default "/Game/Data/Inputs/IA_Sprint.IA_Sprint"))
  (bind _charactermovement (`self.CharacterMovement`))
  ;[0.6301 1 0.6446] Настройка анимации бега
  (:`Triggered`
    ;;[0.8283 0.4362 1] Бег
    (set `CharacterMovementComponent.MaxWalkSpeed` 400.0 _charactermovement))
  (:`Canceled`
    ;;[0.08369 0.3832 1] Хотьба
    (set `CharacterMovementComponent.MaxWalkSpeed` 200.0 _charactermovement :!label _label_4))
  (:`Completed`
    (goto _label_4)))

(fn `AmmoCounter`
  ;[0 0.9702 1] Подсчет количества потронов
  (set `self.Ammo` (`KismetMathLibrary.Clamp` (- (`self.Ammo`) 1) 0 60)))

(fn `LineTrace`
  (bind _returnvalue (`GameplayStatics.GetPlayerCameraManager` 0))
  (bind _returnvalue_2 (`self.K2_GetActorLocation` _returnvalue))
  ;[1 0.9844 0.02818] Line trace стрельба
  (bind _outhit (`KismetSystemLibrary.LineTraceSingle` _returnvalue_2 (+ _returnvalue_2 (* 50000.0 (`self.GetActorForwardVector` _returnvalue))) "TraceTypeQuery1"))
  (bind (_bblockinghit _binitialoverlap _time _distance _location _impactpoint _normal _impactnormal _physmat _hitactor _hitcomponent _hitbonename _bonename _hititem _elementindex _faceindex _tracestart _traceend) (`GameplayStatics.BreakHitResult` _outhit))
  ;;[0 0.8779 1] Проверка чтобы ровно из дула автомата
  (if _bblockinghit
    (`KismetSystemLibrary.LineTraceSingle` (`SceneComponent.K2_GetComponentLocation` (`/Game/FPS_Weapon_Bundle/BP_Weapon.Arrow` (`self.BP_Weapon`))) _impactpoint "TraceTypeQuery1")
    (else
      (`KismetSystemLibrary.LineTraceSingle` (`SceneComponent.K2_GetComponentLocation` (`/Game/FPS_Weapon_Bundle/BP_Weapon.Arrow` (`self.BP_Weapon`))) _traceend "TraceTypeQuery1"))))

(fn `UserConstructionScript`)