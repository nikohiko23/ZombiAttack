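; Zombie enemy Blueprint that chases the player's SWAT character from BeginPlay.
; A looping 0.1-second timer re-fires MoveToCharacter, which calls AIMoveTo using the player reference and location fetched by a helper function.
; On success it flags the player as reached, halts movement and re-enters the chase.
; On failure it waits briefly, clears the flag and cancels the stored timer.
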(event `self.ReceiveBeginPlay`
  (`self.MoveToCharacter`))

(event `MoveToCharacter`
  ;[0.3936 1 0.9502] Логика зомби
  (bind _returnvalue (`KismetSystemLibrary.K2_SetTimerDelegate` (delegate `MoveToCharacter`) 0.1 true true :!label _label))
  (set `self.TimerMoveToCharacter` _returnvalue)
  (`|AIMoveTo` self (`self.Func_MoveToCharacter`) (`self.BP_Swat_Character`) 20.0
    (:`OnSuccess`
      (set `self.BoolGetCharacter` true)
      (`MovementComponent.StopMovementImmediately` (`self.CharacterMovement`))
      (goto _label))
    (:`OnFail`
      (`KismetSystemLibrary.Delay` 1.0)
      (set `self.BoolGetCharacter` false)
      (`KismetSystemLibrary.K2_ClearAndInvalidateTimerHandle` (`self.TimerMoveToCharacter`)))))

(fn `Func_MoveToCharacter`
  (returns (CharacterLocation :type "Vector Structure"))
  ;[1 0.6079 0.7189] Получаем местонахождение персонажа для зомби
  (bind _output_get (set `self.BP_Swat_Character` (cast `/Game/MainCharacter/BP_SwatCharacter` (`GameplayStatics.GetPlayerCharacter` 0) :!pure true)))
  (bind _output_get_2 (set `self.PlayerLocation` (`self.K2_GetActorLocation` _output_get)))
  (return _output_get_2))

(fn `UserConstructionScript`)