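; Zombie enemy that chases the player's SWAT character and dies as a physics ragdoll.
; MoveToCharacter re-issues AI Move To through a looping timer, deactivating movement to play a montage and flag the character as caught.
; A failed move reactivates movement, then after a delay clears the flag and timer.
; Damage feeds health straight into the widget bar's percent; at zero, capsule collision turns off and the widget is destroyed.
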(event `self.ReceiveAnyDamage`
  (params (Damage :type "Float (single-precision)") (DamageType :type "DamageType Object Reference") (InstigatedBy :type "Controller Object Reference") (DamageCauser :type "Actor Object Reference"))
  (bind _ac_health (`self.AC_Health`))
  (bind _widget (`self.Widget`))
  (bind _mesh (`self.Mesh`))
  ;[0.3936 1 0.9502] Логика зомби
  ;;[1 0.164 0] Логика поподания по зомби и отнятия Hp
  (bind _output_get (set `/Game/Data/AC_Health.Health` (- (`/Game/Data/AC_Health.Health` _ac_health) Damage) _ac_health))
  (`ProgressBar.SetPercent` (`/Game/Data/Widgets/WBP_ZombiHealthBar.PB_HealthZombi` (`self.WBP Zombi Health Bar`)) _output_get)
  (if (<= _output_get 0.0)
    (`PrimitiveComponent.SetCollisionEnabled` (`self.CapsuleComponent`) "NoCollision")
    (`PrimitiveComponent.SetCollisionEnabled` _mesh "QueryAndPhysics")
    (`PrimitiveComponent.SetSimulatePhysics` _mesh true)
    (`/Engine/EditorBlueprintResources/StandardMacros.IsValid` _widget
      (:`Is Valid`
        (`ActorComponent.K2_DestroyComponent` _widget)))))

(event `self.ReceiveBeginPlay`
  ;[0.3936 1 0.9502] Логика зомби
  (`self.MoveToCharacter`)
  (bind _aswbp_zombi_health_bar (cast `/Game/Data/Widgets/WBP_ZombiHealthBar` (`WidgetComponent.GetUserWidgetObject` (`self.Widget`))))
  (set `self.WBP Zombi Health Bar` _aswbp_zombi_health_bar))

(event `MoveToCharacter`
  ;[0.3936 1 0.9502] Логика зомби
  (bind _returnvalue (`KismetSystemLibrary.K2_SetTimerDelegate` (delegate `MoveToCharacter`) 0.1 true true :!label _label))
  (set `self.TimerMoveToCharacter` _returnvalue)
  (`|AIMoveTo` self (`self.Func_MoveToCharacter`) (`self.BP_Swat_Character`) 35.0
    (:`then`
      (`ActorComponent.Deactivate` (`self.CharacterMovement`))
      (`|PlayMontage` (`self.Mesh`)
        (:`then`
          (set `self.BoolGetCharacter` true)
          (goto _label))))
    (:`OnFail`
      (`ActorComponent.Activate` (`self.CharacterMovement`) false)
      (`KismetSystemLibrary.Delay` 1.0)
      (set `self.BoolGetCharacter` false)
      (`KismetSystemLibrary.K2_ClearAndInvalidateTimerHandle` (`self.TimerMoveToCharacter`)))))

(fn `Func_MoveToCharacter`
  (returns (CharacterLocation :type "Vector Structure"))
  ;[1 0.6079 0.7189] Получаем местонахождение персонажа для зомби
  (bind _output_get (set `self.BP_Swat_Character` (cast `/Game/MainCharacter/BP_SwatCharacter` (`GameplayStatics.GetPlayerCharacter` 0) :!pure true)))
  (bind _output_get_2 (set `self.PlayerLocation` (`self.K2_GetActorLocation` _output_get)))
  (return _output_get_2))

(fn `UserConstructionScript`)